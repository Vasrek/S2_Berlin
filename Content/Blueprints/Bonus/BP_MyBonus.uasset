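; BP_MyBonus is a pickup that gives the player health or ammo, depending on its bonus type.
; The construction script shows a sphere mesh for Medic and a cube for Munitions.
; When a BP_MyPlayer overlaps the collision, it calls AddHealth or AddAmmo, then hides the actor and disables collision.
; After a ten-second delay it re-enables collision and visibility, so the pickup respawns in place.
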(event `self.Collision.OnComponentBeginOverlap`
  (params (OverlappedComponent :type "PrimitiveComponent Object Reference") (OtherActor :type "Actor Object Reference") (OtherComp :type "PrimitiveComponent Object Reference") (OtherBodyIndex :type Integer) (bFromSweep :type Boolean) (SweepResult :type "HitResult Structure (by ref)"))
  ;[1 1 1] Add ammo or health (depends on the type bonus) - hide it and deactivate collisions after 10 seconds re enable everything
  (bind _asbp_my_player (cast `/Game/Blueprints/Player/BP_MyPlayer` OtherActor))
  (switch `/Game/Blueprints/Bonus/E_BonusType` (`self.E_BonusTypes`)
    (:`NewEnumerator0`
      (`/Game/Blueprints/Player/BP_MyPlayer.AddHealth` _asbp_my_player (`self.nbHealthToAdd`)))
    (:`NewEnumerator1`
      (`/Game/Blueprints/Player/BP_MyPlayer.AddAmmo` _asbp_my_player (`self.nbAmmoToAdd`))))
  (`PrimitiveComponent.SetCollisionEnabled` (`self.Collision`) "NoCollision")
  (`self.SetActorHiddenInGame` true)
  (`KismetSystemLibrary.Delay` 10.0)
  (`PrimitiveComponent.SetCollisionEnabled` (`self.Collision`) "QueryOnly")
  (`self.SetActorHiddenInGame` false))

(fn `UserConstructionScript`
  (switch `/Game/Blueprints/Bonus/E_BonusType` (`self.E_BonusTypes`)
    (:`NewEnumerator0`
      (`StaticMeshComponent.SetStaticMesh` (`self.Mesh`) "/Game/StarterContent/Shapes/Shape_Sphere.Shape_Sphere"))
    (:`NewEnumerator1`
      (`StaticMeshComponent.SetStaticMesh` (`self.Mesh`) "/Game/StarterContent/Shapes/Shape_Cube.Shape_Cube"))))