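; Game mode that runs an endless wave system, spawning BP_MyFirstAI enemies in waves that double in size.
; The player's HUD runs the timer between waves and calls back through a bound event to spawn the next one.
; Enemies spawn at randomly picked TargetPoints, and each death event decrements the kill counter.
; The HUD count refreshes on each change, and the timer restarts when none remain.
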(event `self.ReceiveBeginPlay`
  (bind _hud_ref (`/Game/Blueprints/Player/BP_MyPlayer.HUD_REF` (`self.PlayerRef`)))
  (`KismetSystemLibrary.Delay` 0.2)
  (bind _asbp_my_player (cast `/Game/Blueprints/Player/BP_MyPlayer` (`GameplayStatics.GetPlayerCharacter` 0)))
  (set `self.PlayerRef` _asbp_my_player)
  (`/Game/Blueprints/Widgets/WBP_HUD.StartTimerBetweenWaves` _hud_ref)
  (add `/Game/Blueprints/Widgets/WBP_HUD.SpawnANewWave` _hud_ref (delegate `CallSpawnWave`)))

(event `CallSpawnWave`
  (if (`self.FirstWave?`)
    (set `self.FirstWave?` false)
    (set `self.nbEnnemiesToSpawn` 2)
    (`self.SpawnWave` 2)
    (else
      (bind _output_get (set `self.nbEnnemiesToSpawn` (* (`self.nbEnnemiesToSpawn`) 2)))
      (`self.SpawnWave` _output_get))))

(event `SpawnWave`
  (params (nbEnnemiesToSpawn :type Integer))
  (set `self.nbEnnemiesToSpawn` nbEnnemiesToSpawn)
  (set `self.nbEnnemiesToKill` (`self.nbEnnemiesToSpawn`))
  (`/Game/Blueprints/Widgets/WBP_HUD.UpdateEnnemiesLeftTokill` (`/Game/Blueprints/Player/BP_MyPlayer.HUD_REF` (`self.PlayerRef`)))
  (bind _outactors (`GameplayStatics.GetAllActorsOfClass` "/Script/Engine.TargetPoint"))
  (for _ (range (`self.nbEnnemiesToSpawn`))
    (bind (_returnvalue_location _returnvalue_rotation) (`KismetMathLibrary.BreakTransform` (`SceneComponent.K2_GetComponentToWorld` (`TargetPoint.SpriteComponent` (`KismetArrayLibrary.Array_Random` _outactors)))))
    (bind _returnvalue (`|SpawnActorFromClass` "/Game/Blueprints/IA/BP_MyFirstAI.BP_MyFirstAI_C" (`KismetMathLibrary.MakeTransform` _returnvalue_location _returnvalue_rotation) "AlwaysSpawn" "MultiplyWithRoot" null null))
    (add `/Game/Blueprints/IA/BP_MyFirstAI.AIDeath` _returnvalue (delegate `DecreasedEnnemiesLeftToKill`))))

(event `DecreasedEnnemiesLeftToKill`
  (bind _hud_ref (`/Game/Blueprints/Player/BP_MyPlayer.HUD_REF` (`self.PlayerRef`)))
  (bind _result (`/Engine/EditorBlueprintResources/StandardMacros.DecrementInt` (`self.nbEnnemiesToKill`))
    (:`  `
      (if (== _result 0)
        (`/Game/Blueprints/Widgets/WBP_HUD.UpdateEnnemiesLeftTokill` _hud_ref)
        (`/Game/Blueprints/Widgets/WBP_HUD.StartTimerBetweenWaves` _hud_ref)
        (else
          (`/Game/Blueprints/Widgets/WBP_HUD.UpdateEnnemiesLeftTokill` (`/Game/Blueprints/Player/BP_MyPlayer.HUD_REF` (`self.PlayerRef`))))))))

(fn `UserConstructionScript`)